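; Brick block for a Bomberman-style level that is destroyed by bomb explosions and may drop a power-up.
; On the block explosion event, a chance check decides whether to spawn a pickup, then the actor destroys itself after a short delay.
; The spawn picks a random type and maps it to a bomb, speed, detonator or fire pickup class, placed at the block's location.
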(event `self.OnBlockExplosion`
  (if (`self.CanSpawnPickuableByChance`)
    (`self.SpawnPickupable`))
  (`KismetSystemLibrary.Delay` 0.2)
  (`self.K2_DestroyActor`))

(fn `SpawnPickupable`
  (locals (SpawnClass :type "Actor Class Reference" :default "BlueprintGeneratedClass'/Game/Blueprints/Level/PickupBP.PickupBP_C'"))
  (set `local.SpawnClass` (select `SpawnType` (`self.GetRandomSpawnType`) :`SP_BombIncrease` "/Game/Blueprints/Level/PickupBP_BombIncrease.PickupBP_BombIncrease_C" :`SP_WalkSpeed` "/Game/Blueprints/Level/PickupBP_Speed.PickupBP_Speed_C" :`SP_Detonator` "/Game/Blueprints/Level/PickupBP_Detonator.PickupBP_Detonator_C" :`SP_FireIncrease` "/Game/Blueprints/Level/PickupBP_FireIncrease.PickupBP_FireIncrease_C" :!type "Actor Class Reference"))
  (`|SpawnActorFromClass` (`local.SpawnClass`) (`KismetMathLibrary.MakeTransform` (`self.K2_GetActorLocation`)) "Undefined" "OverrideRootScale" null null))

(fn `UserConstructionScript`)